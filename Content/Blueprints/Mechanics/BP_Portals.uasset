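; BP_Portals is a pair of linked blue and red portals in one actor that teleport tagged actors between each other.
; Overlapping either box with an actor tagged "Portal" plays a sound at the actor's origin and moves it to the opposite portal's exit point without sweeping.
; A held BP_Object is first detached from its player through DetachObject, so it travels through alone.
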(event `self.bluebox.OnComponentBeginOverlap`
  (params (OverlappedComponent :type "PrimitiveComponent Object Reference") (OtherActor :type "Actor Object Reference") (OtherComp :type "PrimitiveComponent Object Reference") (OtherBodyIndex :type Integer) (bFromSweep :type Boolean) (SweepResult :type "HitResult Structure (by ref)"))
  (if (`self.ActorHasTag` OtherActor "Portal")
    (`GameplayStatics.PlaySoundAtLocation` "/Game/Audio/SFX/PortalSound.PortalSound" (`self.K2_GetActorLocation`) (struct) 1.0 1.0 0.0 null null null null)
    (bind _asbp_object (cast `/Game/Blueprints/Mechanics/BP_Object` OtherActor)
      (:`then`
        (if (`/Game/Blueprints/Mechanics/BP_Object.Held?` _asbp_object)
          (`/Game/ThirdPerson/Blueprints/BP_ThirdPersonCharacter.DetachObject` (`/Game/Blueprints/Mechanics/BP_Object.player` _asbp_object)))
        (`self.K2_SetActorLocation` _asbp_object (`SceneComponent.K2_GetComponentLocation` (`self.RedPoint`)) false true))
      (:`CastFailed`
        (`self.K2_SetActorLocation` OtherActor (`SceneComponent.K2_GetComponentLocation` (`self.RedPoint`)) false true)))))

(event `self.redbox.OnComponentBeginOverlap`
  (params (OverlappedComponent :type "PrimitiveComponent Object Reference") (OtherActor :type "Actor Object Reference") (OtherComp :type "PrimitiveComponent Object Reference") (OtherBodyIndex :type Integer) (bFromSweep :type Boolean) (SweepResult :type "HitResult Structure (by ref)"))
  (if (`self.ActorHasTag` OtherActor "Portal")
    (`GameplayStatics.PlaySoundAtLocation` "/Game/Audio/SFX/PortalSound.PortalSound" (`self.K2_GetActorLocation`) (struct) 1.0 1.0 0.0 null null null null)
    (bind _asbp_object (cast `/Game/Blueprints/Mechanics/BP_Object` OtherActor)
      (:`then`
        (if (`/Game/Blueprints/Mechanics/BP_Object.Held?` _asbp_object)
          (`/Game/ThirdPerson/Blueprints/BP_ThirdPersonCharacter.DetachObject` (`/Game/Blueprints/Mechanics/BP_Object.player` _asbp_object)))
        (`self.K2_SetActorLocation` _asbp_object (`SceneComponent.K2_GetComponentLocation` (`self.BluePoint`)) false true))
      (:`CastFailed`
        (`self.K2_SetActorLocation` OtherActor (`SceneComponent.K2_GetComponentLocation` (`self.BluePoint`)) false true)))))

(fn `UserConstructionScript`)