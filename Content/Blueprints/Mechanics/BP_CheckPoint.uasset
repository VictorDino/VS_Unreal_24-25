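; BP_CheckPoint is a checkpoint actor that records a transform on the player character when they overlap its box trigger.
; On overlap by BP_ThirdPersonCharacter, it plays a sound and writes CheckpointTransform from a point raised above the cylinder, the arrow's rotation and the cylinder's scale.
; It then switches the cylinder to a white glow material, with no guard against repeat triggering.
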(event `self.Box.OnComponentBeginOverlap`
  (params (OverlappedComponent :type "PrimitiveComponent Object Reference") (OtherActor :type "Actor Object Reference") (OtherComp :type "PrimitiveComponent Object Reference") (OtherBodyIndex :type Integer) (bFromSweep :type Boolean) (SweepResult :type "HitResult Structure (by ref)"))
  (bind (_returnvalue_location _returnvalue_rotation _returnvalue_scale) (`KismetMathLibrary.BreakTransform` (`SceneComponent.K2_GetComponentToWorld` (`self.Cylinder`))))
  (bind _asbp_third_person_character (cast `/Game/ThirdPerson/Blueprints/BP_ThirdPersonCharacter` OtherActor))
  (`GameplayStatics.PlaySoundAtLocation` "/Game/Audio/SFX/ChekpointSound.ChekpointSound" (`self.K2_GetActorLocation`) (struct) 1.0 1.0 0.0 null null null null)
  (set `/Game/ThirdPerson/Blueprints/BP_ThirdPersonCharacter.CheckpointTransform` (`KismetMathLibrary.MakeTransform` (+ _returnvalue_location (0.0 0.0 300.0)) (`SceneComponent.K2_GetComponentRotation` (`self.Arrow`)) _returnvalue_scale) _asbp_third_person_character)
  (`PrimitiveComponent.SetMaterial` (`self.Cylinder`) 0 "/Game/Materials/MAT_SmoothWhiteGlow.MAT_SmoothWhiteGlow"))

(fn `UserConstructionScript`)