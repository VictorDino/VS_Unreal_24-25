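; BP_MechanicalPlatform is a platform that moves to a target location when activated and returns to its start when deactivated.
; Activate and Deactivate flip an Active flag, and the start location is cached from the actor at BeginPlay.
; Each event runs a next-tick loop that eases the static mesh with VInterpTo, without sweep, until it arrives or the flag flips, allowing mid-travel reversal.
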(event `self.ReceiveBeginPlay`
  (set `self.StartLocation` (`self.K2_GetActorLocation`)))

(event `Activate`
  (bind _staticmesh (`self.StaticMesh`))
  (bind _returnvalue (`SceneComponent.K2_GetComponentLocation` _staticmesh))
  (if (not (`self.Active`))
    (set `self.Active` true)
    (`SceneComponent.K2_SetWorldLocation` _staticmesh (`KismetMathLibrary.VInterpTo` _returnvalue (`self.TargetLocation`) (`GameplayStatics.GetWorldDeltaSeconds`) (`self.Speed`)) false false :!label _label)
    (if (and (not (== _returnvalue (`self.TargetLocation`))) (`self.Active`))
      (`KismetSystemLibrary.DelayUntilNextTick`)
      (goto _label))))

(event `Deactivate`
  (bind _staticmesh (`self.StaticMesh`))
  (bind _returnvalue (`SceneComponent.K2_GetComponentLocation` _staticmesh))
  (if (`self.Active`)
    (set `self.Active` false)
    (`SceneComponent.K2_SetWorldLocation` _staticmesh (`KismetMathLibrary.VInterpTo` _returnvalue (`self.StartLocation`) (`GameplayStatics.GetWorldDeltaSeconds`) (`self.Speed`)) false false :!label _label_2)
    (if (and (not (== _returnvalue (`self.StartLocation`))) (not (`self.Active`)))
      (`KismetSystemLibrary.DelayUntilNextTick`)
      (goto _label_2))))

(fn `UserConstructionScript`)